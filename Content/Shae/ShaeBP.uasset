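; Blueprint for the character Shae, who walks back and forth between Initial and Final positions once ShaeStartWalk is called.
; A hardcoded chain of latent MoveComponentTo and Delay nodes eases the root along each leg, pauses, then rotates it around with Box collision disabled.
; IsWalking tracks moving versus paused states.
; The chain does not loop: it stops after the third leg's turn with collision still off, leaving duplicated follow-on segments unconnected.
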(event `ShaeStartWalk`
  (bind _rootcomponent (`self.RootComponent`))
  (bind _box (`self.Box`))
  (bind _rootcomponent_2 (`self.RootComponent`))
  ;[1 1 1] Shae Walk
  (set `self.shae_walk` true)
  (set `self.is_walking?` true)
  (`KismetSystemLibrary.MoveComponentTo` _rootcomponent (`self.final`) (struct) true true 18.0)
  (set `self.is_walking?` false)
  (`KismetSystemLibrary.Delay` 5.0)
  (`PrimitiveComponent.SetCollisionEnabled` _box "NoCollision")
  (`KismetSystemLibrary.MoveComponentTo` _rootcomponent (`self.final`) (struct :`Yaw` 180.0) false false 1.0)
  (`KismetSystemLibrary.Delay` 1.0)
  (set `self.is_walking?` true)
  (`PrimitiveComponent.SetCollisionEnabled` _box "QueryAndPhysics")
  (`KismetSystemLibrary.MoveComponentTo` _rootcomponent (`self.initial`) (struct :`Yaw` 180.0) true false 18.0)
  (set `self.is_walking?` false)
  (`KismetSystemLibrary.Delay` 5.0)
  (`PrimitiveComponent.SetCollisionEnabled` _box "NoCollision")
  (`KismetSystemLibrary.MoveComponentTo` _rootcomponent (`self.initial`) (struct) false false 1.0)
  (`KismetSystemLibrary.Delay` 1.0)
  (`PrimitiveComponent.SetCollisionEnabled` _box "QueryAndPhysics")
  (set `self.is_walking?` true)
  (`KismetSystemLibrary.MoveComponentTo` _rootcomponent_2 (`self.final`) (struct) true true 18.0)
  (set `self.is_walking?` false)
  (`KismetSystemLibrary.Delay` 5.0)
  (`PrimitiveComponent.SetCollisionEnabled` (`self.Box`) "NoCollision")
  (`KismetSystemLibrary.MoveComponentTo` _rootcomponent_2 (`self.final`) (struct :`Yaw` 180.0) false false 1.0)
  (`KismetSystemLibrary.Delay` 1.0))

(fn `UserConstructionScript`)